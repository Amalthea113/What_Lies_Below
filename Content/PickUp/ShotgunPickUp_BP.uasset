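; Shotgun pickup actor that gives the player a timed shotgun weapon when its sphere is overlapped by a Player-tagged actor.
; It updates the MainCharacter HUD, stops firing, switches off the other special weapons and sets a slower fire rate, reverting fire rate and shotgun state after a delay.
; The cube is removed immediately, while the actor waits out the same duration before destroying itself.
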(event OnComponentBeginOverlap(Sphere)
  (params (OverlappedComponent :type Primitive%20Component%20Object%20Reference) (OtherActor :type Actor%20Object%20Reference) (OtherComp :type Primitive%20Component%20Object%20Reference) (OtherBodyIndex :type Integer) (bFromSweep :type Boolean) (SweepResult :type Hit%20Result%20Structure%20%28by%20ref%29))
  (if (Actor|ActorHasTag OtherActor "Player")
    (Utilities|FlowControl|Sequence
      (:then_0
        (bind _asmain_character (Utilities|Casting|CastToMainCharacter OtherActor))
        (Default|SetShotgun (Variables|/Game/TopDown/Blueprints/MainCharacter.MainCharacter_C|GetHUD _asmain_character))
        (Default|StopFiring _asmain_character)
        (Variables|/Game/TopDown/Blueprints/MainCharacter.MainCharacter_C|SetGrenadeLauncherActive _asmain_character false)
        (Variables|/Game/TopDown/Blueprints/MainCharacter.MainCharacter_C|SetMinigunActive _asmain_character false)
        (Variables|/Game/TopDown/Blueprints/MainCharacter.MainCharacter_C|SetShotgunActive _asmain_character true)
        (Variables|/Game/TopDown/Blueprints/MainCharacter.MainCharacter_C|SetFireRate _asmain_character 0.5)
        (Utilities|FlowControl|Delay 5.0)
        (Default|StopFiring _asmain_character)
        (Variables|/Game/TopDown/Blueprints/MainCharacter.MainCharacter_C|SetFireRate _asmain_character 0.15)
        (Variables|/Game/TopDown/Blueprints/MainCharacter.MainCharacter_C|SetShotgunActive _asmain_character false))
      (:then_1
        (Components|DestroyComponent (Variables|Default|GetCube))
        (Utilities|FlowControl|Delay 5.0)
        (Actor|DestroyActor)))))

(event EventBeginPlay)

(event Collision|EventActorBeginOverlap
  (params (OtherActor :type Actor%20Object%20Reference)))

(event EventTick
  (params (DeltaSeconds :type Float%20%28single-precision%29)))

(fn ConstructionScript)