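; HealthKit_BP is a health pickup that heals the player on overlap.
; Its Sphere overlap event checks for the Player tag and casts to MainCharacter.
; If Health is below the cap, it adds a fixed amount clamped to that cap, then destroys itself; at full health the kit stays in the world.
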(event OnComponentBeginOverlap(Sphere)
  (params (OverlappedComponent :type Primitive%20Component%20Object%20Reference) (OtherActor :type Actor%20Object%20Reference) (OtherComp :type Primitive%20Component%20Object%20Reference) (OtherBodyIndex :type Integer) (bFromSweep :type Boolean) (SweepResult :type Hit%20Result%20Structure%20%28by%20ref%29))
  (if (Actor|ActorHasTag OtherActor "Player")
    (bind _asmain_character (Utilities|Casting|CastToMainCharacter OtherActor))
    (if (not (>= (Variables|/Game/TopDown/Blueprints/MainCharacter.MainCharacter_C|GetHealth _asmain_character) 2.5e+02))
      (Variables|/Game/TopDown/Blueprints/MainCharacter.MainCharacter_C|SetHealth _asmain_character (Math|Float|Clamp(Float) (+ (Variables|/Game/TopDown/Blueprints/MainCharacter.MainCharacter_C|GetHealth _asmain_character) 1e+02) 0.0 2.5e+02))
      (Actor|DestroyActor))))

(event EventBeginPlay)

(event Collision|EventActorBeginOverlap
  (params (OtherActor :type Actor%20Object%20Reference)))

(event EventTick
  (params (DeltaSeconds :type Float%20%28single-precision%29)))

(fn ConstructionScript)