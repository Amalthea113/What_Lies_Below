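; DamageBoost_BP is a pickup that temporarily powers up the player.
; When a Player-tagged actor overlaps its Sphere, a sequence sets PoweredUp on the MainCharacter, then clears it after a fifteen-second delay.
; A second branch destroys the Cube immediately but delays destroying the actor for the same duration.
; The Sphere is never disabled, so it can still receive overlaps during that window.
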(event OnComponentBeginOverlap(Sphere)
  (params (OverlappedComponent :type Primitive%20Component%20Object%20Reference) (OtherActor :type Actor%20Object%20Reference) (OtherComp :type Primitive%20Component%20Object%20Reference) (OtherBodyIndex :type Integer) (bFromSweep :type Boolean) (SweepResult :type Hit%20Result%20Structure%20%28by%20ref%29))
  (if (Actor|ActorHasTag OtherActor "Player")
    (Utilities|FlowControl|Sequence
      (:then_0
        (bind _asmain_character (Utilities|Casting|CastToMainCharacter OtherActor))
        (Variables|/Game/TopDown/Blueprints/MainCharacter.MainCharacter_C|SetPoweredUp _asmain_character true)
        (Utilities|FlowControl|Delay 15.0)
        (Variables|/Game/TopDown/Blueprints/MainCharacter.MainCharacter_C|SetPoweredUp _asmain_character false))
      (:then_1
        (Components|DestroyComponent (Variables|Default|GetCube))
        (Utilities|FlowControl|Delay 15.0)
        (Actor|DestroyActor)))))

(event EventBeginPlay)

(event Collision|EventActorBeginOverlap
  (params (OtherActor :type Actor%20Object%20Reference)))

(event EventTick
  (params (DeltaSeconds :type Float%20%28single-precision%29)))

(fn ConstructionScript)