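; BP_MissileRobot is an AI enemy robot with a gun and a missile launch attack, revealing its body and rifle meshes shortly after BeginPlay.
; ShootGun fires two quick projectiles, while MissileLaunchAttack spawns an upward-shooting missile with an explosion effect.
; Death detaches the controller, stops blocking pawns and a custom channel, and runs a timeline-driven dissolve on dynamic materials before destroying the actor.
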(event Custom|Dissolving
  (bind _mesh (Variables|Character|GetMesh))
  (bind _returnvalue (Rendering|Material|CreateDynamicMaterialInstance (Variables|Default|GetStaticMesh) 0 "/Game/Assets/Models/Weapons/Basic_Rifle/Rifle_mat.Rifle_mat" "None" :!class /Script/Engine.PrimitiveComponent))
  (bind _returnvalue_2 (Rendering|Material|CreateDynamicMaterialInstance _mesh 0 "/Game/Assets/Models/Characters/Beefy_Boy/Robot_Body_V2.Robot_Body_V2" "None" :!class /Script/Engine.PrimitiveComponent))
  (bind _returnvalue_3 (Rendering|Material|CreateDynamicMaterialInstance _mesh 1 "/Game/Assets/Models/Characters/Beefy_Boy/Beefy2.Beefy2" "None" :!class /Script/Engine.PrimitiveComponent))
  (bind _returnvalue_4 (Rendering|Material|CreateDynamicMaterialInstance _mesh 2 "/Game/Assets/Models/Characters/Beefy_Boy/Robot_Pack_V2.Robot_Pack_V2" "None" :!class /Script/Engine.PrimitiveComponent))
  (bind _returnvalue_5 (Rendering|Material|CreateDynamicMaterialInstance _mesh 3 "/Game/Assets/Models/Characters/Beefy_Boy/Beefy3.Beefy3" "None" :!class /Script/Engine.PrimitiveComponent))
  (bind _newtrack_0 (Timeline|Timeline_0 Play)
    (:Update
      (Rendering|Material|SetScalarParameterValue _returnvalue_3 "Dissolve" _newtrack_0 :!class /Script/Engine.MaterialInstanceDynamic)
      (Utilities|FlowControl|Delay 1.26)
      (Actor|DestroyActor))))

(event EventBeginPlay
  (Utilities|FlowControl|Delay 2.25)
  (Development|SetHiddeninGame (Variables|Default|GetStaticMesh) false false)
  (Development|SetHiddeninGame (Variables|Character|GetMesh) false false))

(event EventDeath
  (bind _capsulecomponent (Variables|Default|GetCapsuleComponent))
  (Class|Pawn|DetachfromControllerPendingDestroy)
  (CallFunction|Dissolving)
  (Collision|SetCollisionResponsetoChannel _capsulecomponent "ECC_Pawn" "ECR_Ignore")
  (Collision|SetCollisionResponsetoChannel _capsulecomponent "ECC_GameTraceChannel1" "ECR_Ignore"))

(event EventShootGun
  (bind _projetilespawnpoint (Variables|Default|GetProjetileSpawnPoint))
  (bind _returnvalue (Transformation|GetWorldTransform _projetilespawnpoint))
  (Audio|PlaySoundatLocation "/Game/Audio/MissileRobot_GunShot.MissileRobot_GunShot" "0, 0, 0" "0, 0, 0" 1.0 1.0 0.0 0 0 0 0)
  (Game|SpawnActorfromClass "/Game/AI/MissileRobot/EnemyProjectile.EnemyProjectile_C" (Math|Transform|MakeTransform (.location _returnvalue) (.rotation _returnvalue) "0.400000,0.400000,0.400000") "AlwaysSpawn" 0 0)
  (Utilities|FlowControl|Delay 0.2)
  (Game|SpawnActorfromClass "/Game/AI/MissileRobot/EnemyProjectile.EnemyProjectile_C" (Math|Transform|MakeTransform (.location _returnvalue) (.rotation _returnvalue) "0.400000,0.400000,0.400000") "AlwaysSpawn" 0 0))

(event EventMissileLaunchAttack
  (bind _missilespawnpoint (Variables|Default|GetMissileSpawnPoint))
  (bind _returnvalue (Transformation|GetWorldTransform _missilespawnpoint))
  (Audio|PlaySoundatLocation "/Game/Audio/MissileLaunch.MissileLaunch" "0, 0, 0" "0, 0, 0" 1.0 1.0 0.0 0 0 0 0)
  (Game|SpawnActorfromClass "/Game/AI/MissileRobot/MissileShootingUp.MissileShootingUp_C" (Math|Transform|MakeTransform (.location _returnvalue) (.rotation _returnvalue) "1.000000,1.000000,1.000000") "AlwaysSpawn" 0 0)
  (Effects|SpawnEmitteratLocation "/Game/StarterContent/Particles/P_Explosion.P_Explosion" (.location _returnvalue) (.rotation _returnvalue) "0.700000,0.700000,0.700000"))

(fn ConstructionScript
  (|CallParentFunction))