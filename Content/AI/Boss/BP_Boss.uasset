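; Boss enemy that tracks its health phase, turns toward the player and fires a sci-fi rifle projectile.
; Damage starts a self-recalling Delay loop for yaw facing, stores the player in the Blackboard, broadcasts health changes and picks one of three health-threshold phases.
; SpawnBar adds the boss widget once, and FireSciFiRifle spawns projectiles at the muzzle.
; Other weapon and enrage events are empty, and the phase switch is unconnected.
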(event Custom|Fire%20Grenade%20Launcher)

(event Custom|Fire%20MiniGun)

(event Custom|Fire%20Shotgun)

(event Custom|Fire%20SciFi%20Rifle
  (bind _rifleshotspot (Variables|Default|GetRifleShotSpot))
  (bind _returnvalue (Transformation|GetWorldTransform _rifleshotspot))
  (Audio|PlaySoundatLocation "/Game/Audio/MissileRobot_GunShot.MissileRobot_GunShot" "0, 0, 0" "0, 0, 0" 1.0 0.8 0.0 0 0 0 0)
  (Game|SpawnActorfromClass "/Game/AI/MissileRobot/BossProjectile.BossProjectile_C" (Math|Transform|MakeTransform (.location _returnvalue) (.rotation _returnvalue) "0.700000,0.700000,0.700000") "AlwaysSpawn" 0 0))

(event Custom|Enraged)

(event Custom|Face%20Player
  (Utilities|IsValid self
    (:Is%20Valid
      (Transformation|SetActorRelativeRotation (Math|Rotator|MakeRotator 0.0 0.0 (.yaw (Math|Rotator|FindLookatRotation (Transformation|GetActorLocation) (Transformation|GetActorLocation (Game|GetPlayerCharacter 0))))))
      (Utilities|FlowControl|Delay 0.01)
      (CallFunction|FacePlayer))))

(event Custom|SpawnBar
  (Utilities|FlowControl|DoOnce false
    (:Completed
      (bind _returnvalue (UserInterface|CreateWidget "/Game/TopDown/Blueprints/AntennaTower/Boss_Widget.Boss_Widget_C"))
      (bind _output_get (Variables|Default|SetNewVar_0 _returnvalue))
      ;[0 1 0.4732] Any Damage & Health
      (UserInterface|Viewport|AddtoViewport _output_get 0))))

(event Game|Damage|EventAnyDamage
  (params (Damage :type Float%20%28single-precision%29) (DamageType :type Damage%20Type%20Object%20Reference) (InstigatedBy :type Controller%20Object%20Reference) (DamageCauser :type Actor%20Object%20Reference))
  ;[0 1 0.4732] Any Damage & Health
  (CallFunction|FacePlayer)
  (AI|Components|Blackboard|SetValueasObject (AI|GetBlackboard 0) (Utilities|Name|MakeLiteralName "PlayerActor") (Game|GetPlayerCharacter 0))
  (bind _output_get (Variables|Default|SetHealth (- (Variables|Default|GetHealth) Damage)))
  (Default|CallOnHealthChange _output_get)
  (if (>= _output_get 7.5e+03)
    (Development|PrintString (Utilities|String|ToString(Float) _output_get))
    (Variables|Default|SetCurrentPhase "NewEnumerator0")
    (elif (and (< _output_get 7.5e+03) (>= _output_get 5e+03))
      (Development|PrintString (Utilities|String|ToString(Float) _output_get))
      (Variables|Default|SetCurrentPhase "NewEnumerator1")
      (elif (and (< _output_get 5e+03) (> _output_get 0.0))
        (Development|PrintString (Utilities|String|ToString(Float) _output_get))
        (Variables|Default|SetCurrentPhase "NewEnumerator2")))))

(fn ConstructionScript)